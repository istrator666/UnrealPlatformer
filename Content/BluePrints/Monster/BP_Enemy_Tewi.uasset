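; BP_Enemy_Tewi is a 2D Paper flipbook enemy that patrols via InterpToMovement, flipping its sprite when the path reverses.
; A player overlapping the Box launches upward and stomps it dead, while overlapping the Capsule kills the player.
; Any damage costs fixed HP and briefly pauses movement with a hurt flipbook, or triggers death at zero.
; Death disables collision, stops movement, plays sound and animation, awards score through BP_GameInstance, then expires.
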(event `self.InterpToMovement.OnInterpToReverse`
  (params (ImpactResult :type "HitResult Structure (by ref)") (Time :type "Float (single-precision)"))
  (bind _paperflipbook (`self.PaperFlipbook`))
  (`/Engine/EditorBlueprintResources/StandardMacros.FlipFlop`
    (:`A`
      (`SceneComponent.K2_SetRelativeRotation` _paperflipbook (struct :`Yaw` 180.0) false false))
    (:`B`
      (`SceneComponent.K2_SetRelativeRotation` :`self` _paperflipbook))))

(event `self.Box.OnComponentBeginOverlap`
  (params (OverlappedComponent :type "PrimitiveComponent Object Reference") (OtherActor :type "Actor Object Reference") (OtherComp :type "PrimitiveComponent Object Reference") (OtherBodyIndex :type Integer) (bFromSweep :type Boolean) (SweepResult :type "HitResult Structure (by ref)"))
  (bind _asbp_player (cast `/Game/BluePrints/Player/BP_Player` OtherActor))
  (`Character.LaunchCharacter` _asbp_player (0.0 0.0 480.0) false true)
  (`self.Death`))

(event `Death`
  (`self.SetActorEnableCollision` false)
  (`PaperFlipbookComponent.SetFlipbook` (`self.PaperFlipbook`) "/Game/FilpBook/Tewi_Filpbook/Tewi_Death.Tewi_Death")
  (`ActorComponent.SetComponentTickEnabled` (`self.InterpToMovement`) false)
  (`GameplayStatics.PlaySound2D` "/Game/Sound/SE/SE_Stomp.SE_Stomp" 1.0 1.0 0.0 null null)
  (bind _asbp_game_instance (cast `/Game/GameMode/BP_GameInstance` (`GameplayStatics.GetGameInstance`)))
  (`/Game/GameMode/BP_GameInstance.ScoreCountChack` _asbp_game_instance 200)
  (`KismetSystemLibrary.Delay` 0.3)
  (`PaperFlipbookComponent.Stop` (`self.PaperFlipbook`))
  (`self.SetLifeSpan` 2.0))

(event `self.Capsule.OnComponentBeginOverlap`
  (params (OverlappedComponent :type "PrimitiveComponent Object Reference") (OtherActor :type "Actor Object Reference") (OtherComp :type "PrimitiveComponent Object Reference") (OtherBodyIndex :type Integer) (bFromSweep :type Boolean) (SweepResult :type "HitResult Structure (by ref)"))
  (bind _asbp_player (cast `/Game/BluePrints/Player/BP_Player` OtherActor))
  (`/Game/BluePrints/Player/BP_Player.Death` _asbp_player))

(event `self.ReceiveAnyDamage`
  (params (Damage :type "Float (single-precision)") (DamageType :type "DamageType Object Reference") (InstigatedBy :type "Controller Object Reference") (DamageCauser :type "Actor Object Reference"))
  (`ActorComponent.SetComponentTickEnabled` (`self.InterpToMovement`) false)
  (`PaperFlipbookComponent.SetFlipbook` (`self.PaperFlipbook`) "/Game/FilpBook/Tewi_Filpbook/Tewi_TakeDamage.Tewi_TakeDamage")
  (`GameplayStatics.PlaySound2D` "/Game/Sound/SE/SE_Hit.SE_Hit" 1.0 1.0 0.0 null null)
  (set `self.HP` (- (`self.HP`) 3))
  (if (> (`self.HP`) 0)
    (`KismetSystemLibrary.RetriggerableDelay` 0.4)
    (`PaperFlipbookComponent.SetFlipbook` (`self.PaperFlipbook`) "/Game/FilpBook/Tewi_Filpbook/Tewi_Walk.Tewi_Walk")
    (`ActorComponent.SetComponentTickEnabled` (`self.InterpToMovement`) true)
    (else
      (`KismetSystemLibrary.RetriggerableDelay` 0.1)
      (`self.Death`))))

(fn `UserConstructionScript`)