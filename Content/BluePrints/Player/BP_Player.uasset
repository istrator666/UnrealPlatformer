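; BP_Player is the 2D side-scrolling player character (Cirno) with Enhanced Input movement, jumping, ice shooting, ladders and wall sliding/jumping.
; A self-repeating timer picks the flipbook from state flags, water and velocity, while Tick keeps the spring arm on the player.
; Wall contact slows falling and launches jumps off the hit normal; down input briefly enables a bottom box.
; Death and level clear load levels, using the GameInstance for lives and restart location.
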(event `self.ReceiveBeginPlay`
  ;[1 1 1] 동기화 및 Controller 세팅
  (`ActorComponent.SetIsReplicated` (`self.Sprite`) true)
  (bind `_as플레이어_컨트롤러` (cast `PlayerController` (`self.GetController`)))
  (`EnhancedInputSubsystemInterface.AddMappingContext` (pcsubsystem `EnhancedInputLocalPlayerSubsystem` `_as플레이어_컨트롤러`) "/Game/Player/input/IMC_default.IMC_default" 0 (struct))
  (`self.CameraSet`)
  (`PrimitiveComponent.SetCollisionEnabled` (`self.Box_Bottom`) "NoCollision")
  (`self.RestartBegin`)
  (`self.UpdateAnimation`))

(event `self.ReceiveTick`
  (params (DeltaSeconds :type "Float (single-precision)"))
  ;[1 1 1] Tick
  (`self.CameraPos`))

(event `UpdateAnimation`
  (bind (_returnvalue_x _returnvalue_y _returnvalue_z) (`KismetMathLibrary.BreakVector` (`self.GetVelocity`)))
  (bind _returnvalue (`NavMovementComponent.IsFalling` (`self.CharacterMovement`)))
  (bind _returnvalue_2 (< _returnvalue_z -100.0))
  (bind _returnvalue_3 (> (`KismetMathLibrary.VSize` (`self.GetVelocity`)) 0.0))
  ;[1 1 1] 애니메이션 관리
  (`KismetSystemLibrary.K2_SetTimerDelegate` (delegate `UpdateAnimation`) 0.01)
  (if (`self.bDeath`)
    (set `self.AnimSet` 5)
    (elif (`self.bShot`)
      (set `self.AnimSet` 4)
      (elif (`self.bLadder`)
        (set `self.AnimSet` 6)
        (elif (`self.bWallGrab`)
          (set `self.AnimSet` 11)
          (elif (`self.bWater`)
            (if _returnvalue
              (if _returnvalue_2
                (set `self.AnimSet` 10)
                (else
                  (set `self.AnimSet` 9)))
              (elif _returnvalue_3
                (set `self.AnimSet` 8)
                (else
                  (set `self.AnimSet` 7))))
            (elif _returnvalue
              (if _returnvalue_2
                (set `self.AnimSet` 3)
                (else
                  (set `self.AnimSet` 2)))
              (elif _returnvalue_3
                (set `self.AnimSet` 1)
                (else
                  (set `self.AnimSet` 0)))))))))
  (`PaperFlipbookComponent.SetFlipbook` (`self.Sprite`) (select `int` (`self.AnimSet`) :`0` "/Game/FilpBook/Crino_Filpbook/free_cirno_idle.free_cirno_idle" :`1` "/Game/FilpBook/Crino_Filpbook/free_cirno_walk.free_cirno_walk" :`2` "/Game/FilpBook/Crino_Filpbook/free_cirno_jump.free_cirno_jump" :`3` "/Game/FilpBook/Crino_Filpbook/free_cirno_fall.free_cirno_fall" :`4` "/Game/FilpBook/Crino_Filpbook/Cirno_Attack.Cirno_Attack" :`5` "/Game/FilpBook/Crino_Filpbook/free_cirno_Death.free_cirno_Death" :`6` "/Game/FilpBook/Crino_Filpbook/free_cirno25_Ladder.free_cirno25_Ladder" :`7` "/Game/FilpBook/Crino_Filpbook/cirno_water_idle.cirno_water_idle" :`8` "/Game/FilpBook/Crino_Filpbook/cirno_water_walk.cirno_water_walk" :`9` "/Game/FilpBook/Crino_Filpbook/cirno_water_jump.cirno_water_jump" :`10` "/Game/FilpBook/Crino_Filpbook/cirno_water_fall.cirno_water_fall" :`11` "/Game/FilpBook/Crino_Filpbook/cirno_wall_2.cirno_wall_2" :!type "PaperFlipbook Object Reference")))

(event `LevelClear`
  ;[1 1 1] Level Clear
  (set `self.bClear` true)
  (`CharacterMovementComponent.DisableMovement` (`self.CharacterMovement`))
  (`KismetSystemLibrary.Delay` 3.0)
  (`GameplayStatics.OpenLevel` "Level02"))

(event `CameraPos`
  (bind (_returnvalue_x _returnvalue_y _returnvalue_z) (`KismetMathLibrary.BreakVector` (`self.K2_GetActorLocation`)))
  (bind (_returnvalue_x_2 _returnvalue_y_2 _returnvalue_z_2) (`KismetMathLibrary.BreakVector` (`self.K2_GetActorLocation`)))
  ;[1 1 1] 카메라 위치
  (switch `int` (`self.CamType`)
    (:`0`
      (`SceneComponent.K2_SetWorldLocation` (`self.SpringArm`) (`KismetMathLibrary.MakeVector` _returnvalue_x_2 _returnvalue_y_2 _returnvalue_z_2) false false))
    (:`1`
      (`SceneComponent.K2_SetWorldLocation` (`self.SpringArm`) (`KismetMathLibrary.MakeVector` _returnvalue_x _returnvalue_y _returnvalue_z) false false))))

(event `CameraSet`
  ;[1 1 1] CameraSet
  (switch `int` (`self.CamType`)
    (:`0`
      (set `SpringArmComponent.SocketOffset` (0.0 0.0 75.0) (`self.SpringArm`)))))

(event `CamZMove`
  (params (NewCamZ :type "Float (double-precision)"))
  ;[1 1 1] CamZMove
  (bind (_direction _alpha) (`Timeline|CamZTimeline` :!via `PlayFromStart`)
    (:`Update`
      (set `self.TimelineAlpha` _alpha)
      (set `self.CamZ` (`KismetMathLibrary.Lerp` (`self.CamZ`) NewCamZ (`self.TimelineAlpha`))))))

(event `RestartBegin`
  (bind _restart_location (`/Game/GameMode/BP_GameInstance.Restart_Location` (cast `/Game/GameMode/BP_GameInstance` (`GameplayStatics.GetGameInstance`) :!pure true)))
  ;[1 1 1] RestartBegin
  (if (`KismetMathLibrary.NotEqualExactly_VectorVector` _restart_location)
    (`self.K2_SetActorLocation` _restart_location)))

(event `EnhancedInput|/Game/Player/input/IA_Move`
  (params (ActionValue :type "Float (double-precision)") (ElapsedSeconds :type "Float (double-precision)") (TriggeredSeconds :type "Float (double-precision)") (InputAction :type "InputAction Object Reference" :default "/Game/Player/input/IA_Move.IA_Move"))
  ;[1 1 1] 좌우 이동
  (:`Triggered`
    (if (`self.bLadder`)
      (`self.AddMovementInput` (0.3 0.0 0.0) ActionValue)
      (else
        (`self.AddMovementInput` (1.0 0.0 0.0) ActionValue)))
    (`self.WallJumpMove`)
    (`self.Update_FlipSprite`)))

(event `Update_FlipSprite`
  ;[1 1 1] A, D 스프라이트 좌우 반전 함수
  (`/Engine/EditorBlueprintResources/StandardMacros.CompareFloat` (.x (`MovementComponent.Velocity` (`self.GetMovementComponent`)))
    (:`>`
      (`SceneComponent.K2_SetWorldRotation` :`self` (`self.Sprite`)))
    (:`<`
      (`SceneComponent.K2_SetWorldRotation` (`self.Sprite`) (struct :`Yaw` 180.0) false false))))

(event `EnhancedInput|/Game/Player/input/IA_Jump`
  (params (ActionValue :type Boolean) (ElapsedSeconds :type "Float (double-precision)") (TriggeredSeconds :type "Float (double-precision)") (InputAction :type "InputAction Object Reference" :default "/Game/Player/input/IA_Jump.IA_Jump"))
  (bind _bhitnormal_x (`KismetMathLibrary.BreakVector` (`self.bHitNormal`)))
  ;[1 1 1] 점프
  (:`Triggered`
    (if (`self.bLadder`)
      (set `self.bLadder` false)
      (`CharacterMovementComponent.SetMovementMode` (`self.CharacterMovement`) "MOVE_Walking" 0)
      (`self.Jump`)
      (elif (`NavMovementComponent.IsFalling` (`self.CharacterMovement`))
        (if (`self.bWallGrab`)
          (`self.LaunchCharacter` (`KismetMathLibrary.MakeVector` (* _bhitnormal_x 300.0) 0.0 (`CharacterMovementComponent.JumpZVelocity` (`self.CharacterMovement`))) false true)
          (set `self.bWallGrab` false))
        (else
          (`self.Jump`)))))
  (:`Completed`
    (`self.StopJumping`)))

(event `Death`
  ;[1 1 1] 사망
  (set `self.bDeath` true)
  (`CharacterMovementComponent.DisableMovement` (`self.CharacterMovement`))
  (`GameplayStatics.PlaySound2D` "/Game/Sound/SE/SE_Pichun.SE_Pichun" 1.0 1.0 0.0 null null)
  (`self.SetActorEnableCollision` false)
  (`KismetSystemLibrary.Delay` 0.3)
  (bind _asbp_game_instance (cast `/Game/GameMode/BP_GameInstance` (`GameplayStatics.GetGameInstance`)))
  (`/Game/GameMode/BP_GameInstance.LifeCountCheck` _asbp_game_instance)
  (if (>= (`/Game/GameMode/BP_GameInstance.Life_Count` _asbp_game_instance) 0)
    (`KismetSystemLibrary.Delay` 1.0)
    (`KismetSystemLibrary.ExecuteConsoleCommand` "RestartLevel" null)
    (else
      (`KismetSystemLibrary.Delay` 1.0)
      (`GameplayStatics.OpenLevel` "GameOver"))))

(event `EnhancedInput|/Game/Player/input/IA_Shot`
  (params (ActionValue :type Boolean) (ElapsedSeconds :type "Float (double-precision)") (TriggeredSeconds :type "Float (double-precision)") (InputAction :type "InputAction Object Reference" :default "/Game/Player/input/IA_Shot.IA_Shot"))
  ;[1 1 1] 투사체
  (:`Triggered`
    (if (`self.bDeath`)
      _
      (elif (not (`self.bShot`))
        (set `self.bShot` true)
        (`self.UpdateAnimation`)
        (`|SpawnActorFromClass` "/Game/BluePrints/Player/BP_CirnoProjectile.BP_CirnoProjectile_C" (`SceneComponent.K2_GetComponentToWorld` (`self.IceProjectile`)) "Undefined" "OverrideRootScale" null null)
        (`GameplayStatics.PlaySound2D` "/Game/Sound/SE/SE_Shoot.SE_Shoot" 1.0 1.0 0.0 null null)
        (`KismetSystemLibrary.RetriggerableDelay` 0.5)
        (set `self.bShot` false)))))

(event `LadderMove`
  (bind _returnvalue (`|GetInputActionValue`))
  ;[1 1 1] 사다리 이동 함수
  (if (`self.bOnLadder`)
    (if (!= _returnvalue 0.0)
      (set `self.bLadder` true)
      (`CharacterMovementComponent.SetMovementMode` (`self.CharacterMovement`) "MOVE_Flying" 0)
      (`self.AddMovementInput` (0.0 0.0 0.3) _returnvalue)
      (`PaperFlipbookComponent.SetPlayRate` (`self.Sprite`) 1.0)
      (else
        (`PaperFlipbookComponent.SetPlayRate` (`self.Sprite`) 0.0)))
    (else
      (set `self.bLadder` false)
      (`PaperFlipbookComponent.SetPlayRate` (`self.Sprite`) 1.0))))

(event `ChainFloor`
  ;[1 1 1] ChainFloor 함수
  (if (>= (`|GetInputActionValue`) 0.0)
    (`PrimitiveComponent.SetCollisionEnabled` (`self.Box_Bottom`) "NoCollision")
    (else
      (`PrimitiveComponent.SetCollisionEnabled` (`self.Box_Bottom`) "QueryOnly")
      (`KismetSystemLibrary.RetriggerableDelay` 0.2)
      (`PrimitiveComponent.SetCollisionEnabled` (`self.Box_Bottom`) "NoCollision"))))

(event `EnhancedInput|/Game/Player/input/IA_MoveUp`
  (params (ActionValue :type "Float (double-precision)") (ElapsedSeconds :type "Float (double-precision)") (TriggeredSeconds :type "Float (double-precision)") (InputAction :type "InputAction Object Reference" :default "/Game/Player/input/IA_MoveUp.IA_MoveUp"))
  ;[1 1 1] 사다리
  (:`Triggered`
    (`self.ChainFloor`)
    (`self.LadderMove`)))

(event `self.ReceiveHit`
  (params (MyComp :type "PrimitiveComponent Object Reference") (Other :type "Actor Object Reference") (OtherComp :type "PrimitiveComponent Object Reference") (bSelfMoved :type Boolean) (HitLocation :type "Vector Structure") (HitNormal :type "Vector Structure") (NormalImpulse :type "Vector Structure") (Hit :type "HitResult Structure (by ref)"))
  ;[1 1 1] 벽 점프
  (bind _output_get (set `self.bHitNormal` HitNormal))
  (if (!= (.x _output_get) 0.0)
    (if (`self.bOnWall`)
      (set `self.bWallGrab` true))
    (else
      (set `self.bWallGrab` false))))

(event `self.Box_Wall.OnComponentBeginOverlap`
  (params (OverlappedComponent :type "PrimitiveComponent Object Reference") (OtherActor :type "Actor Object Reference") (OtherComp :type "PrimitiveComponent Object Reference") (OtherBodyIndex :type Integer) (bFromSweep :type Boolean) (SweepResult :type "HitResult Structure (by ref)"))
  ;[1 1 1] 벽 점프
  (set `self.bOnWall` true))

(event `self.Box_Wall.OnComponentEndOverlap`
  (params (OverlappedComponent :type "PrimitiveComponent Object Reference") (OtherActor :type "Actor Object Reference") (OtherComp :type "PrimitiveComponent Object Reference") (OtherBodyIndex :type Integer))
  ;[1 1 1] 벽 점프
  (set `self.bWallGrab` false)
  (set `self.bOnWall` false))

(event `WallJumpMove`
  (bind (_returnvalue_x _returnvalue_y _returnvalue_z) (`KismetMathLibrary.BreakVector` (`self.GetVelocity`)))
  ;[1 1 1] 벽 점프
  (if (`self.bWallGrab`)
    (if (>= _returnvalue_z 0.0)
      (set `CharacterMovementComponent.GravityScale` 1.0 (`self.CharacterMovement`))
      (else
        (set `CharacterMovementComponent.GravityScale` 0.25 (`self.CharacterMovement`))
        (`/Engine/EditorBlueprintResources/StandardMacros.DoOnce` false :!label _label
          (:`Completed`
            (`NiagaraFunctionLibrary.SpawnSystemAtLocation` "/Game/Particle/NG_WallSide.NG_WallSide" (`SceneComponent.K2_GetComponentLocation` (`self.PT_Pos`)))
            (`KismetSystemLibrary.Delay` 0.05)
            (goto _label :!via `Reset`)))))
    (else
      (set `CharacterMovementComponent.GravityScale` 1.0 (`self.CharacterMovement`)))))

(event `EnhancedInput|/Game/Player/input/IA_Pause`
  (params (ActionValue :type Boolean) (ElapsedSeconds :type "Float (double-precision)") (TriggeredSeconds :type "Float (double-precision)") (InputAction :type "InputAction Object Reference" :default "/Game/Player/input/IA_Pause.IA_Pause"))
  ;[1 1 1] Pause
  (:`Triggered`
    (bind _asbp_game_mode (cast `/Game/GameMode/BP_GameMode` (`GameplayStatics.GetGameMode`)))
    (`/Game/GameMode/BP_GameMode.Pause_HUD` _asbp_game_mode)))

(fn `UserConstructionScript`)