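; BP_Ladder is a climbable ladder built from Paper2D sprites with an adjustable height.
; The construction script stacks non-colliding sprites from LadderHeight and stretches the ScaleZ component vertically to match.
; Actor overlap sets the player's OnLadder flag on entry.
; On exit it clears OnLadder and Ladder and returns the player's movement mode to Walking, leaving climbing itself to BP_Player.
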(event `self.ReceiveActorBeginOverlap`
  (params (OtherActor :type "Actor Object Reference"))
  (bind _asbp_player (cast `/Game/BluePrints/Player/BP_Player` OtherActor))
  (set `/Game/BluePrints/Player/BP_Player.bOnLadder` true _asbp_player))

(event `self.ReceiveActorEndOverlap`
  (params (OtherActor :type "Actor Object Reference"))
  (bind _asbp_player (cast `/Game/BluePrints/Player/BP_Player` OtherActor))
  (set `/Game/BluePrints/Player/BP_Player.bOnLadder` false _asbp_player)
  (set `/Game/BluePrints/Player/BP_Player.bLadder` false _asbp_player)
  (`CharacterMovementComponent.SetMovementMode` (`Character.CharacterMovement` _asbp_player) "MOVE_Walking" 0))

(fn `UserConstructionScript`
  (for _index (range (+ (`self.Ladder_Height`) 1))
    (bind _returnvalue (`AddComponent|NODE_AddPaperSpriteComponent-0` :`RelativeTransform` (`KismetMathLibrary.MakeTransform` (`KismetMathLibrary.MakeVector` 0.0 -1.0 (* _index 48.0)) (struct) (3.0 3.0 3.0))))
    (`PrimitiveComponent.SetCollisionEnabled` _returnvalue "NoCollision")
    (`SceneComponent.SetRelativeScale3D` (`self.ScaleZ`) (`KismetMathLibrary.MakeVector` 1.0 1.0 (`KismetMathLibrary.Conv_IntToDouble` (+ (`self.Ladder_Height`) 1))))))