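; BP_Water is a water volume that switches BP_Player into a swimming-like state while it overlaps.
; On begin overlap it stops the player, sets its Water flag, lowers gravity, jump velocity and walk speed, allows near-unlimited jumps, and tints the sprite blue.
; On end overlap it restores hardcoded defaults rather than the player's previous values.
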(event `self.ReceiveActorBeginOverlap`
  (params (OtherActor :type "Actor Object Reference"))
  (bind _asbp_player (cast `/Game/BluePrints/Player/BP_Player` OtherActor))
  (set `/Game/BluePrints/Player/BP_Player.bWater` true _asbp_player)
  (bind _charactermovement (`Character.CharacterMovement` _asbp_player))
  (set `CharacterMovementComponent.GravityScale` 0.3 _charactermovement)
  (set `CharacterMovementComponent.JumpZVelocity` 240.0 _charactermovement)
  (set `CharacterMovementComponent.MaxWalkSpeed` 200.0 _charactermovement)
  (`MovementComponent.StopMovementImmediately` _charactermovement)
  (set `Character.JumpMaxCount` 99 _asbp_player)
  (`PaperFlipbookComponent.SetSpriteColor` (`PaperCharacter.Sprite` _asbp_player) (struct :`R` 0.169629 :`G` 0.497967 :`B` 0.930111 :`A` 1.0)))

(event `self.ReceiveActorEndOverlap`
  (params (OtherActor :type "Actor Object Reference"))
  (bind _asbp_player (cast `/Game/BluePrints/Player/BP_Player` OtherActor))
  (set `/Game/BluePrints/Player/BP_Player.bWater` false _asbp_player)
  (bind _charactermovement (`Character.CharacterMovement` _asbp_player))
  (set `CharacterMovementComponent.GravityScale` 1.0 _charactermovement)
  (set `CharacterMovementComponent.JumpZVelocity` 480.0 _charactermovement)
  (set `CharacterMovementComponent.MaxWalkSpeed` 600.0 _charactermovement)
  (set `Character.JumpMaxCount` 1 _asbp_player)
  (`PaperFlipbookComponent.SetSpriteColor` (`PaperCharacter.Sprite` _asbp_player) (struct :`R` 0.930111 :`G` 0.930111 :`B` 0.930111 :`A` 1.0)))

(fn `UserConstructionScript`)