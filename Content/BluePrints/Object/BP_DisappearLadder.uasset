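; BP_DisappearLadder is a Paper2D ladder that repeatedly appears and disappears on a fixed cycle.
; After a configurable StartTime delay, a fast looping timer drives a DoOnce gate that makes the sprite visible and collidable, then hidden and non-colliding, for three seconds each.
; A Box overlap tracks whether BP_Player is nearby, so the appearance sound plays only while the player is inside it.
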(event `self.ReceiveBeginPlay`
  (`PrimitiveComponent.SetCollisionEnabled` (`self.PaperSprite`) "NoCollision")
  (`KismetSystemLibrary.Delay` (`self.StartTime`))
  (`KismetSystemLibrary.K2_SetTimer` null "Loop" 0.1 true)
  (if (`PrimitiveComponent.IsOverlappingActor` (`self.Box`) (cast `/Game/BluePrints/Player/BP_Player` (`GameplayStatics.GetPlayerPawn` 0) :!pure true))
    (set `self.bSound` true)))

(event `Loop`
  (`/Engine/EditorBlueprintResources/StandardMacros.DoOnce` false :!label _label
    (:`Completed`
      (`SceneComponent.SetHiddenInGame` (`self.PaperSprite`) false false)
      (`PrimitiveComponent.SetCollisionEnabled` (`self.PaperSprite`) "QueryAndPhysics")
      (if (`self.bSound`)
        (`GameplayStatics.PlaySound2D` "/Game/Sound/SE/SE_Kieruasiba.SE_Kieruasiba" 1.0 1.0 0.0 null null))
      (`KismetSystemLibrary.Delay` 3.0)
      (`SceneComponent.SetHiddenInGame` (`self.PaperSprite`) true false)
      (`PrimitiveComponent.SetCollisionEnabled` (`self.PaperSprite`) "NoCollision")
      (`KismetSystemLibrary.Delay` 3.0)
      (goto _label :!via `Reset`))))

(event `self.ReceiveTick`
  (params (DeltaSeconds :type "Float (single-precision)")))

(event `self.Box.OnComponentBeginOverlap`
  (params (OverlappedComponent :type "PrimitiveComponent Object Reference") (OtherActor :type "Actor Object Reference") (OtherComp :type "PrimitiveComponent Object Reference") (OtherBodyIndex :type Integer) (bFromSweep :type Boolean) (SweepResult :type "HitResult Structure (by ref)"))
  (cast `/Game/BluePrints/Player/BP_Player` OtherActor)
  (set `self.bSound` true))

(event `self.Box.OnComponentEndOverlap`
  (params (OverlappedComponent :type "PrimitiveComponent Object Reference") (OtherActor :type "Actor Object Reference") (OtherComp :type "PrimitiveComponent Object Reference") (OtherBodyIndex :type Integer))
  (cast `/Game/BluePrints/Player/BP_Player` OtherActor)
  (set `self.bSound` false))

(fn `UserConstructionScript`)