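; BP_GameMode is the game mode that manages the main side-view HUD and the pause toggle.
; BeginPlay creates HUD_2DSide and adds it to the viewport.
; Pause_HUD flips the paused state, clears all widgets, then creates either a pause widget or a fresh HUD_2DSide, and plays a pause sound.
; An unconnected console command for showing collision is left in the graph.
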(event `self.ReceiveBeginPlay`
  (bind _returnvalue (`|CreateWidget` "/Game/UI/HUD_2DSide.HUD_2DSide_C"))
  (`UserWidget.AddToViewport` _returnvalue 0))

(event `Pause_HUD`
  (if (`GameplayStatics.IsGamePaused`)
    (`GameplayStatics.SetGamePaused` false)
    (`WidgetLayoutLibrary.RemoveAllWidgets`)
    (bind _returnvalue (`|CreateWidget` "/Game/UI/HUD_2DSide.HUD_2DSide_C"))
    (`UserWidget.AddToViewport` _returnvalue 0)
    (else
      (`GameplayStatics.SetGamePaused` true)
      (`WidgetLayoutLibrary.RemoveAllWidgets`)
      (bind _returnvalue_2 (`|CreateWidget` "/Game/UI/HUD_Puase.HUD_Puase_C"))
      (`UserWidget.AddToViewport` _returnvalue_2 0)))
  (`GameplayStatics.PlaySound2D` "/Game/Sound/SE/SE_Pause.SE_Pause" 1.0 1.0 0.0 null null))

(fn `UserConstructionScript`)